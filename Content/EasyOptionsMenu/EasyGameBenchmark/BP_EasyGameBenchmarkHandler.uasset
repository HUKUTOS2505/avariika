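; Level actor that runs a game benchmark when the game instance flags one as requested, recording frame times while a level sequence plays.
; On BeginPlay it waits a tick, shows the overlay, disables player input and starts the sequence.
; Start and pause events toggle Tick, which stores every delta time and sends every tenth to the overlay.
; Ending stops the sequence, shows a results widget, updates the game instance and unpauses for chart display.
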(event `self.ReceiveBeginPlay`
  ;[0.2 0.2 1] Init
  (bind _benchmarkrequested_ (message `/Game/EasyOptionsMenu/EasyGameUI/Utilities/BPI_EGUI_GameInstanceInterface.HasGameBenchmarkBeenRequested?` (`GameplayStatics.GetGameInstance`)))
  (if _benchmarkrequested_
    (`KismetSystemLibrary.DelayUntilNextTick`)
    (`self.InitBenchmark`)))

(event `InitBenchmark`
  (bind _output (`|ConvertAsset` (`self.LevelSequenceToPlay`)))
  ;[0.2 0.2 1] Init
  (`KismetArrayLibrary.Array_Clear` (`self.Frametimes`))
  (bind _returnvalue (`|CreateWidget` "/Game/EasyOptionsMenu/EasyGameBenchmark/WBP_EGB_BenchmarkOverlay.WBP_EGB_BenchmarkOverlay_C" null self))
  (`UserWidget.AddToViewport` _returnvalue 0)
  (set `self.BenchmarkOverlay` _returnvalue)
  (`/Game/EasyOptionsMenu/EasyGameUI/Utilities/BFL_EasyFunctionUtilities.DisableAllInputsOnCharacterAndController`)
  (`/Engine/EditorBlueprintResources/StandardMacros.IsValid` _output
    (:`Is Valid`
      (bind _output_get (set `self.SequencePlayer` (`LevelSequenceActor.SequencePlayer` _output)))
      (`MovieSceneSequencePlayer.Play` _output_get))))

(event `StartBenchmark`
  ;[0.2 1 0.2] Benchmark Controls
  (`self.SetActorTickEnabled` true))

(event `PauseOrResumeBench`
  (params (`Resume?` :type Boolean))
  ;[0.2 1 0.2] Benchmark Controls
  (`self.SetActorTickEnabled` `Resume?`))

(event `EndBenchmark`
  ;[0.2 1 0.2] Benchmark Controls
  (`self.SetActorTickEnabled` false)
  (`Widget.RemoveFromParent` (`self.BenchmarkOverlay`))
  (bind _returnvalue (`|CreateWidget` "/Game/EasyOptionsMenu/EasyGameBenchmark/WBP_EGB_BenchmarkResult.WBP_EGB_BenchmarkResult_C" null (`self.Frametimes`) (`self.TotalFrametimes`)))
  (`UserWidget.AddToViewport` _returnvalue 0)
  (`MovieSceneSequencePlayer.StopAtCurrentTime` (`self.SequencePlayer`))
  (message `/Game/EasyOptionsMenu/EasyGameUI/Utilities/BPI_EGUI_GameInstanceInterface.SetupGameInstanceForGameBenchmark` (`GameplayStatics.GetGameInstance`) true)
  (`GameplayStatics.SetGamePaused` false) ; Force game unpause to ensure \ncharts are displayed properly
)

(event `self.ReceiveTick`
  (params (DeltaSeconds :type "Float (single-precision)"))
  ;[1 0.2 0.2] Frametimes Calculations
  (bind _returnvalue (`KismetArrayLibrary.Array_Add` (`self.Frametimes`) DeltaSeconds))
  (if (== (mod _returnvalue 10) 0)
    (`/Game/EasyOptionsMenu/EasyGameBenchmark/WBP_EGB_BenchmarkOverlay.NewFrametimeValue` (`self.BenchmarkOverlay`) DeltaSeconds))
  (set `self.TotalFrametimes` (+ DeltaSeconds (`self.TotalFrametimes`))))

(fn `UserConstructionScript`)