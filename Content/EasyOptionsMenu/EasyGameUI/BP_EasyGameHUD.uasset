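; HUD Blueprint serving as the central manager for the Easy Options Menu UI and user settings.
; On BeginPlay it loads JSON settings, applies audio and camera FOV, and reads a config asset for input contexts and cursor styling.
; It relays Enhanced Input navigation to registered listener widgets, managing focus, cursor visibility and Escape gating.
; It also opens options, pause and alert widgets, saves settings, and applies upscaling/AA after unpause.
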(event `AudioDeviceSwapped`
  (params (SwapResult :type "SwapAudioOutputResult Structure (by ref)"))
  ;[0.395 1 0.9701 1 40] Init
  ;;[0.395 1 0.9701] User Settings Initialization
)

(event `/Game/EasyOptionsMenu/EasyGameUI/Utilities/BPI_EGUI_HUDInterface.RestoreAudioVolumeSoundModifier`
  ;[0.395 1 0.9701 1 40] Init
  ;;[0.395 1 0.9701] User Settings Initialization
  (`GameplayStatics.PopSoundMixModifier` "/Game/EasyOptionsMenu/DemoContent/Audio/SCM_MasterMix.SCM_MasterMix")
  (`GameplayStatics.PushSoundMixModifier` "/Game/EasyOptionsMenu/DemoContent/Audio/SCM_MasterMix.SCM_MasterMix"))

(event `self.ReceiveBeginPlay`
  ;[0.395 1 0.9701 1 40] Init
  (`parent.ReceiveBeginPlay`)
  ;;[0.395 1 0.9701] User Settings Initialization
  (bind (_outjsonobject _returnvalue) (`JsonBlueprintFunctionLibrary.FromFile` (`/Game/EasyOptionsMenu/EasyGameUI/Utilities/BFL_EasyFunctionUtilities.GetSettingsFilePath`)))
  (bind _output_get (set `self.GlobalUserSettings` _outjsonobject))
  (`/Game/EasyOptionsMenu/EasyGameUI/Utilities/BFL_EasyFunctionUtilities.InitGameInstanceSettings` _output_get _returnvalue)
  (if _returnvalue
    (bind _outvalue (`|GetJsonField` (`self.GlobalUserSettings`) "Audio Device"))
    (`AudioMixerBlueprintLibrary.SwapAudioOutputDevice` _outvalue (delegate `AudioDeviceSwapped`)))
  (`GameplayStatics.PushSoundMixModifier` "/Game/EasyOptionsMenu/DemoContent/Audio/SCM_MasterMix.SCM_MasterMix")
  (`self.UpdatePlayerCameraFOV`)
  (bind _configdataasset (`/Game/EasyOptionsMenu/EasyGameUI/Utilities/BFL_EasyFunctionUtilities.GetConfigDataAsset`))
  (set `self.ConfigDataAsset` _configdataasset)
  (`self.EnableInput` (`self.PlayerOwner`))
  (if (`/Game/EasyOptionsMenu/Core/GlobalConfig/DA_EGUI_GlobalConfig.AddInputMappingContextsOnLevelLoad?` (`self.ConfigDataAsset`))
    (if (`BlueprintMapLibrary.Map_IsEmpty` (`/Game/EasyOptionsMenu/Core/GlobalConfig/DA_EGUI_GlobalConfig.GameplayInputMappingContexts` (`self.ConfigDataAsset`)))
      (`KismetSystemLibrary.PrintString` "Error: A request has been made to add Gameplay Input Mapping Contexts on Level Load, but the array Gameplay Input Mapping Contexts is empty inside the Global Config.  \nThis can cause issues if your character inputs depends on this IMC." true true (struct :`R` 1.0 :`A` 1.0) 60.0))
    (`self.AddAllGameplayInputMappingContexts`))
  (`self.ApplyGlobalCursorStyling`)
  (`KismetSystemLibrary.PrintString` "Easy Game HUD Initialized" true true (struct :`G` 1.0 :`A` 1.0) 5.0))

(event `/Game/EasyOptionsMenu/EasyGameUI/Utilities/BPI_EGUI_HUDInterface.SetAndApplyUpscalingMethods`
  (params (RequestedUpscalingMethod :type "/Game/EasyOptionsMenu/Datas/E_UpscalingMethods Enum" :default "NewEnumerator0") (RequestedAA_Method :type "/Game/EasyOptionsMenu/Datas/E_AntiAliasingMethods Enum" :default "NewEnumerator0"))
  (bind _globalusersettings (`self.GlobalUserSettings`))
  ;[0.3938 1 0.3664 1 40] Upscaling & Anti Aliasing Handling
  (`KismetSystemLibrary.DelayUntilNextTick` :!label _label)
  (if (`GameplayStatics.IsGamePaused`)
    (goto _label)
    (else
      (`/Game/EasyOptionsMenu/EasyGameUI/Utilities/BFL_EasyFunctionUtilities.SetAA AndUpscalingMethods` RequestedUpscalingMethod RequestedAA_Method _globalusersettings)
      (`KismetSystemLibrary.RetriggerableDelay` 0.2) ; Required to avoid crashes
      (`/Game/EasyOptionsMenu/EasyGameUI/Utilities/BFL_EasyFunctionUtilities.ApplyAA AndUpscalingMethod` _globalusersettings))))

(event `/Game/EasyOptionsMenu/EasyGameUI/Utilities/BPI_EGUI_HUDInterface.InitializeFocusHandling`
  (params (WidgetReference :type "UserWidget Object Reference") (InitialElementToFocus :type "Widget Object Reference") (`RegisterInputListener?` :type Boolean) (`SetInputModeGameAndUI?` :type Boolean))
  (bind _playerowner (`self.PlayerOwner`))
  ;[1 0.3176 0.4579 1 40] Handle UI Navigation
  ;;[0.6358 1 0.4314 1 40] UI Navigation Events
  (if `RegisterInputListener?`
    (`/Game/EasyOptionsMenu/EasyGameUI/Utilities/BPI_EGUI_HUDInterface.RegisterInputListener` (`|ConvertAsset` WidgetReference)))
  (if `SetInputModeGameAndUI?`
    (`WidgetBlueprintLibrary.SetInputMode_GameAndUIEx` (`self.PlayerOwner`) null "LockAlways" false true))
  (`/Engine/EditorBlueprintResources/StandardMacros.IsValid` InitialElementToFocus
    (:`Is Valid`
      (`Widget.SetKeyboardFocus` InitialElementToFocus))
    (:`Is Not Valid`
      _))
  (if (`PlayerController.bShowMouseCursor` _playerowner)
    (`/Game/EasyOptionsMenu/EasyGameUI/Utilities/BPI_EGUI_HUDInterface.HandleCursorVisibility` false)
    (else
      (set `PlayerController.bShowMouseCursor` true _playerowner)
      (if (`KismetMathLibrary.NotEqualExactly_Vector2DVector2D` (`self.LastMousePosition`))
        (`PlayerController.SetMouseLocation` (`self.PlayerOwner`) 20 20))
      (`/Game/EasyOptionsMenu/EasyGameUI/Utilities/BPI_EGUI_HUDInterface.HandleCursorVisibility` true)
      (set `self.LostFocus?` false))))

(event `EnhancedInput|/Game/EasyOptionsMenu/EasyGameUI/UINavigation/IA_HeaderNav`
  (params (ActionValue :type "Float (double-precision)") (ElapsedSeconds :type "Float (double-precision)") (TriggeredSeconds :type "Float (double-precision)") (InputAction :type "InputAction Object Reference" :default "/Game/EasyOptionsMenu/EasyGameUI/UINavigation/IA_HeaderNav.IA_HeaderNav"))
  ;[1 0.3176 0.4579 1 40] Handle UI Navigation
  ;;[1 0.3176 0.4579 1 40] UI Navigation Inputs
  (:`Triggered`
    (`self.InputTriggered` "NewEnumerator0" (`KismetStringLibrary.Conv_DoubleToString` ActionValue))))

(event `/Game/EasyOptionsMenu/EasyGameUI/Utilities/BPI_EGUI_HUDInterface.HandleFocusLoss`
  (params (Key :type "Key Structure") (ElementToRefocus :type "Widget Object Reference"))
  ;[1 0.3176 0.4579 1 40] Handle UI Navigation
  ;;[0.6358 1 0.4314 1 40] UI Navigation Events
  (if (or (`KismetInputLibrary.Key_IsGamepadKey` Key) (`KismetInputLibrary.Key_IsKeyboardKey` Key))
    (`/Game/EasyOptionsMenu/EasyGameUI/Utilities/BPI_EGUI_HUDInterface.HandleCursorVisibility` true)
    (if (`self.LostFocus?`)
      (set `self.LostFocus?` false)
      (`/Engine/EditorBlueprintResources/StandardMacros.IsValid` ElementToRefocus
        (:`Is Valid`
          (`Widget.SetKeyboardFocus` ElementToRefocus))))
    (elif (`KismetInputLibrary.Key_IsAxis2D` Key)
      (`/Game/EasyOptionsMenu/EasyGameUI/Utilities/BPI_EGUI_HUDInterface.HandleCursorVisibility` false)
      (else
        (`/Game/EasyOptionsMenu/EasyGameUI/Utilities/BPI_EGUI_HUDInterface.HandleCursorVisibility` false)
        (set `self.LostFocus?` true)))))

(event `/Game/EasyOptionsMenu/EasyGameUI/Utilities/BPI_EGUI_HUDInterface.BlockNavBackUntilEscapeRelease`
  ;[1 0.3176 0.4579 1 40] Handle UI Navigation
  ;;[1 0.3176 0.4579 1 40] UI Navigation Inputs
  (set `self.BlockEscapeUntilRelease?` true)
  (goto _label_2 :!via `Close`))

(event `/Game/EasyOptionsMenu/EasyGameUI/Utilities/BPI_EGUI_HUDInterface.EscapeReleased`
  ;[1 0.3176 0.4579 1 40] Handle UI Navigation
  ;;[1 0.3176 0.4579 1 40] UI Navigation Inputs
  (if (`self.BlockEscapeUntilRelease?`)
    (set `self.BlockEscapeUntilRelease?` false)
    (else
      (goto _label_2 :!via `Open`))))

(event `ApplyGlobalCursorStyling`
  (bind _globalcursorstyling (`/Game/EasyOptionsMenu/Core/GlobalConfig/GlobalStyling/DA_EGUI_GlobalStyling.GlobalCursorStyling` (`/Game/EasyOptionsMenu/Core/GlobalConfig/DA_EGUI_GlobalConfig.StylingDataAsset` (`self.ConfigDataAsset`))))
  ;[0.8363 1 0.3303] Miscellaneous
  (bind _keys (`BlueprintMapLibrary.Map_Keys` _globalcursorstyling))
  (for _array_element _keys
    (bind _class (`|LoadAssetClass` (`BlueprintMapLibrary.Map_Find` _globalcursorstyling _array_element))
      (:`Completed`
        (bind _asuser_widget (castclass `UserWidget` _class))
        (bind _returnvalue (`|CreateWidget` _asuser_widget))
        (`PlayerController.SetMouseCursorWidget` (`self.PlayerOwner`) _array_element _returnvalue)))))

(event `EnhancedInput|/Game/EasyOptionsMenu/EasyGameUI/UINavigation/IA_NavBack`
  (params (ActionValue :type Boolean) (ElapsedSeconds :type "Float (double-precision)") (TriggeredSeconds :type "Float (double-precision)") (InputAction :type "InputAction Object Reference" :default "/Game/EasyOptionsMenu/EasyGameUI/UINavigation/IA_NavBack.IA_NavBack"))
  ;[1 0.3176 0.4579 1 40] Handle UI Navigation
  ;;[1 0.3176 0.4579 1 40] UI Navigation Inputs
  (:`Triggered`
    (`|ExecutionSequence`
      (:`then_0`
        (`/Engine/EditorBlueprintResources/StandardMacros.Gate` true :!label _label_2
          (:`Exit`
            (`self.InputTriggered` "NewEnumerator1"))))
      (:`then_1`
        (goto _label_2 :!via `Open`)))))

(event `/Game/EasyOptionsMenu/EasyGameUI/Utilities/BPI_EGUI_HUDInterface.AddAllGameplayInputMappingContexts`
  (bind _gameplayinputmappingcontexts (`/Game/EasyOptionsMenu/Core/GlobalConfig/DA_EGUI_GlobalConfig.GameplayInputMappingContexts` (`self.ConfigDataAsset`)))
  ;[0.5376 0.1349 1 1 40] Handle Input Mapping Contexts
  (bind _keys (`BlueprintMapLibrary.Map_Keys` _gameplayinputmappingcontexts))
  (for _array_element _keys
    (`EnhancedInputSubsystemInterface.AddMappingContext` (pcsubsystem `EnhancedInputLocalPlayerSubsystem` (`self.PlayerOwner`)) _array_element (`BlueprintMapLibrary.Map_Find` _gameplayinputmappingcontexts _array_element) (struct))))

(event `/Game/EasyOptionsMenu/EasyGameUI/Utilities/BPI_EGUI_HUDInterface.RemoveAllGameplayInputMappingContexts`
  (bind _returnvalue (pcsubsystem `EnhancedInputLocalPlayerSubsystem` (`self.PlayerOwner`)))
  ;[0.5376 0.1349 1 1 40] Handle Input Mapping Contexts
  (bind _keys (`BlueprintMapLibrary.Map_Keys` (`/Game/EasyOptionsMenu/Core/GlobalConfig/DA_EGUI_GlobalConfig.GameplayInputMappingContexts` (`self.ConfigDataAsset`))))
  (for _array_element _keys
    (if (`.ReturnValue` (`EnhancedInputSubsystemInterface.HasMappingContext` _returnvalue _array_element))
      (`EnhancedInputSubsystemInterface.RemoveMappingContext` _returnvalue _array_element (struct))
      (`BlueprintMapLibrary.Map_Add` (`self.GameplayMappingContextsToRestore`) _array_element (`BlueprintMapLibrary.Map_Find` (`/Game/EasyOptionsMenu/Core/GlobalConfig/DA_EGUI_GlobalConfig.GameplayInputMappingContexts` (`self.ConfigDataAsset`)) _array_element)))))

(event `/Game/EasyOptionsMenu/EasyGameUI/Utilities/BPI_EGUI_HUDInterface.HandleCursorVisibility`
  (params (`ShouldHideMouseCursor?` :type Boolean))
  (bind _playerowner (`self.PlayerOwner`))
  (bind _playerowner_2 (`self.PlayerOwner`))
  (bind (_lastmouseposition_x _lastmouseposition_y) (`KismetMathLibrary.BreakVector2D` (`self.LastMousePosition`)))
  (bind (_locationx _locationy) (`PlayerController.GetMousePosition` _playerowner_2))
  (bind (_locationx_2 _locationy_2) (`PlayerController.GetMousePosition` (`self.PlayerOwner`)))
  (bind _bshowmousecursor (`PlayerController.bShowMouseCursor` _playerowner_2))
  ;[1 0.3176 0.4579 1 40] Handle UI Navigation
  ;;[0.6358 1 0.4314 1 40] UI Navigation Events
  (if `ShouldHideMouseCursor?`
    (if _bshowmousecursor
      (if (and (!= _locationx_2 20.0) (!= _locationy_2 20.0))
        (set `self.LastMousePosition` (`KismetMathLibrary.MakeVector2D` _locationx_2 _locationy_2)))
      (set `PlayerController.bShowMouseCursor` false _playerowner)
      (`PlayerController.SetMouseLocation` _playerowner 20 20)
      (bind _output (`self.GetAllValidWidgetsFromHistory`)
        (:`Is Valid`
          (`Widget.SetCursor` _output "None"))))
    (elif (and (not _bshowmousecursor) (!= _locationx 20.0) (!= _locationy 20.0))
      (set `PlayerController.bShowMouseCursor` true _playerowner)
      (`PlayerController.SetMouseLocation` _playerowner (`KismetMathLibrary.FTrunc` _lastmouseposition_x) (`KismetMathLibrary.FTrunc` _lastmouseposition_y))
      (bind _output_2 (`self.GetAllValidWidgetsFromHistory`)
        (:`Is Valid`
          (`Widget.SetCursor` _output_2 "Default"))))))

(event `EnhancedInput|/Game/EasyOptionsMenu/EasyGameUI/UINavigation/IA_NavForward`
  (params (ActionValue :type Boolean) (ElapsedSeconds :type "Float (double-precision)") (TriggeredSeconds :type "Float (double-precision)") (InputAction :type "InputAction Object Reference" :default "/Game/EasyOptionsMenu/EasyGameUI/UINavigation/IA_NavForward.IA_NavForward"))
  ;[1 0.3176 0.4579 1 40] Handle UI Navigation
  ;;[1 0.3176 0.4579 1 40] UI Navigation Inputs
  (:`Triggered`
    (`self.InputTriggered` "NewEnumerator2")))

(event `/Game/EasyOptionsMenu/EasyGameUI/Utilities/BPI_EGUI_HUDInterface.RestoreRemovedGameplayMappingContexts`
  (bind _gameplaymappingcontextstorestore (`self.GameplayMappingContextsToRestore`))
  ;[0.5376 0.1349 1 1 40] Handle Input Mapping Contexts
  (bind _keys (`BlueprintMapLibrary.Map_Keys` _gameplaymappingcontextstorestore))
  (for _array_element _keys
    (`EnhancedInputSubsystemInterface.AddMappingContext` (pcsubsystem `EnhancedInputLocalPlayerSubsystem` (`self.PlayerOwner`)) _array_element (`BlueprintMapLibrary.Map_Find` _gameplaymappingcontextstorestore _array_element) (struct)))
  (`BlueprintMapLibrary.Map_Clear` (`self.GameplayMappingContextsToRestore`)))

(event `/Game/EasyOptionsMenu/EasyGameUI/Utilities/BPI_EGUI_HUDInterface.SetFocusLoss`
  (params (`FocusLost?` :type Boolean))
  ;[1 0.3176 0.4579 1 40] Handle UI Navigation
  ;;[0.6358 1 0.4314 1 40] UI Navigation Events
  (set `self.LostFocus?` `FocusLost?`))

(event `EnhancedInput|/Game/EasyOptionsMenu/EasyGameUI/UINavigation/IA_NavAdditional01`
  (params (ActionValue :type Boolean) (ElapsedSeconds :type "Float (double-precision)") (TriggeredSeconds :type "Float (double-precision)") (InputAction :type "InputAction Object Reference" :default "/Game/EasyOptionsMenu/EasyGameUI/UINavigation/IA_NavAdditional01.IA_NavAdditional01"))
  ;[1 0.3176 0.4579 1 40] Handle UI Navigation
  ;;[1 0.3176 0.4579 1 40] UI Navigation Inputs
  (:`Triggered`
    (`self.InputTriggered` "NewEnumerator3")))

(event `/Game/EasyOptionsMenu/EasyGameUI/Utilities/BPI_EGUI_HUDInterface.CloseAlertBanner`
  (params (UnderlyingWidget :type "UserWidget Object Reference") (ElementToRefocus :type "Widget Object Reference"))
  (bind _alertbannerreference (`self.AlertBannerReference`))
  ;[0.5035 0.4828 1 1 40] Widgets Events/Functions
  (`Widget.SetVisibility` UnderlyingWidget "SelfHitTestInvisible")
  (`/Game/EasyOptionsMenu/EasyGameUI/Utilities/BPI_EGUI_HUDInterface.InitializeFocusHandling` UnderlyingWidget ElementToRefocus (`self.RestoreAsInputListener?`) false)
  (`/Game/EasyOptionsMenu/EasyGameUI/Utilities/BPI_EGUI_HUDInterface.UnregisterInputListener` (`|ConvertAsset` _alertbannerreference))
  (clear `/Game/EasyOptionsMenu/EasyGameUI/CommonWidgets/WBP_EGUI_CommonAlertBanner.ActionRequested` _alertbannerreference)
  (`Widget.SetVisibility` _alertbannerreference "Collapsed"))

(event `EnhancedInput|/Game/EasyOptionsMenu/EasyGameUI/UINavigation/IA_NavAdditional02`
  (params (ActionValue :type Boolean) (ElapsedSeconds :type "Float (double-precision)") (TriggeredSeconds :type "Float (double-precision)") (InputAction :type "InputAction Object Reference" :default "/Game/EasyOptionsMenu/EasyGameUI/UINavigation/IA_NavAdditional02.IA_NavAdditional02"))
  ;[1 0.3176 0.4579 1 40] Handle UI Navigation
  ;;[1 0.3176 0.4579 1 40] UI Navigation Inputs
  (:`Triggered`
    (`self.InputTriggered` "NewEnumerator4")))

(event `/Game/EasyOptionsMenu/EasyGameUI/Utilities/BPI_EGUI_WidgetsCommunicationInterface.OptionsMenuClosedEvent`
  (params (LastActiveTab :type Integer))
  ;[0.5035 0.4828 1 1 40] Widgets Events/Functions
  (set `self.LastOpenedOptionsMenuTab` LastActiveTab)
  (set `self.OptionsMenuRef` null))

(event `/Game/EasyOptionsMenu/EasyGameUI/Utilities/BPI_EGUI_HUDInterface.RegisterInputListener`
  (params (Widget :type "UserWidget Soft Object Reference"))
  (bind _returnvalue (pcsubsystem `EnhancedInputLocalPlayerSubsystem` (`self.PlayerOwner`)))
  ;[1 0.3176 0.4579 1 40] Handle UI Navigation
  ;;[0.6358 1 0.4314 1 40] UI Navigation Events
  ;;;[0.6358 1 0.4314 1 30] Handle Widget Registration
  (`KismetArrayLibrary.Array_AddUnique` (`self.InputListeningWidgets`) Widget)
  (`KismetArrayLibrary.Array_AddUnique` (`self.InputListeningWidgetsHistory`) Widget)
  (if (`PlayerController.WasInputKeyJustPressed` (`self.PlayerOwner`) "Escape")
    (`/Game/EasyOptionsMenu/EasyGameUI/Utilities/BPI_EGUI_HUDInterface.BlockNavBackUntilEscapeRelease`)
    (else
      (`/Game/EasyOptionsMenu/EasyGameUI/Utilities/BPI_EGUI_HUDInterface.EscapeReleased`)))
  (if (not (`.ReturnValue` (`EnhancedInputSubsystemInterface.HasMappingContext` _returnvalue "/Game/EasyOptionsMenu/EasyGameUI/UINavigation/IMC_UI_Navigation.IMC_UI_Navigation")))
    (`EnhancedInputSubsystemInterface.AddMappingContext` _returnvalue "/Game/EasyOptionsMenu/EasyGameUI/UINavigation/IMC_UI_Navigation.IMC_UI_Navigation" 999 (struct))))

(event `EnhancedInput|/Game/EasyOptionsMenu/EasyGameUI/UINavigation/IA_NavAdditional03`
  (params (ActionValue :type Boolean) (ElapsedSeconds :type "Float (double-precision)") (TriggeredSeconds :type "Float (double-precision)") (InputAction :type "InputAction Object Reference" :default "/Game/EasyOptionsMenu/EasyGameUI/UINavigation/IA_NavAdditional03.IA_NavAdditional03"))
  ;[1 0.3176 0.4579 1 40] Handle UI Navigation
  ;;[1 0.3176 0.4579 1 40] UI Navigation Inputs
  (:`Triggered`
    (`self.InputTriggered` "NewEnumerator5")))

(event `/Game/EasyOptionsMenu/EasyGameUI/Utilities/BPI_EGUI_HUDInterface.UnregisterInputListener`
  (params (Widget :type "UserWidget Soft Object Reference"))
  (bind _inputlisteningwidgets (`self.InputListeningWidgets`))
  ;[1 0.3176 0.4579 1 40] Handle UI Navigation
  ;;[0.6358 1 0.4314 1 40] UI Navigation Events
  ;;;[0.6358 1 0.4314 1 30] Handle Widget Registration
  (`KismetArrayLibrary.Array_RemoveItem` _inputlisteningwidgets Widget)
  (if (`KismetArrayLibrary.Array_IsEmpty` _inputlisteningwidgets)
    (`EnhancedInputSubsystemInterface.RemoveMappingContext` (pcsubsystem `EnhancedInputLocalPlayerSubsystem` (`self.PlayerOwner`)) "/Game/EasyOptionsMenu/EasyGameUI/UINavigation/IMC_UI_Navigation.IMC_UI_Navigation" (struct))))

(event `Key|AnyKey` :consume false :paused true :overrideparent false
  (params (Key :type "Key Structure"))
  ;[1 0.3176 0.4579 1 40] Handle UI Navigation
  ;;[1 0.3176 0.4579 1 40] UI Navigation Inputs
  (:`Pressed`
    (bind _output (`self.GetAllValidListeningWidgets`)
      (:`Is Valid`
        (message `/Game/EasyOptionsMenu/EasyGameUI/UINavigation/BPI_InputNavigation.AnyKeyPressed` _output Key))
      (:`Completed`)))
  (:`Released`
    (if (or (== Key "Escape") (`KismetInputLibrary.Key_IsGamepadKey` Key))
      (`/Game/EasyOptionsMenu/EasyGameUI/Utilities/BPI_EGUI_HUDInterface.EscapeReleased`))))

(fn `GetUserSettings`
  (returns (UserSettings :type "JsonObjectWrapper Structure"))
  (return (`self.GlobalUserSettings`)))

(fn `HandleMouseMovementDetection`
  (params (MouseEvent :type "PointerEvent Structure (by ref)") (InstigatorWidget :type "UserWidget Soft Object Reference"))
  (returns (ReturnValue :type "EventReply Structure"))
  (if (> (`KismetMathLibrary.VSize2D` (`KismetInputLibrary.PointerEvent_GetCursorDelta` MouseEvent)) 0.0)
    (if (`KismetArrayLibrary.Array_Contains` (`self.InputListeningWidgets`) (`local.InstigatorWidget`))
      (`/Game/EasyOptionsMenu/EasyGameUI/Utilities/BPI_EGUI_HUDInterface.HandleFocusLoss` "Mouse2D")
      (return (`WidgetBlueprintLibrary.Unhandled`)))))

(fn `InputTriggered`
  (params (InputType :type "/Game/EasyOptionsMenu/EasyGameUI/UINavigation/E_UI_NavInputList Enum" :default "NewEnumerator0") (ActionValue :type String))
  (bind _output (`self.GetAllValidListeningWidgets`)
    (:`Is Valid`
      (message `/Game/EasyOptionsMenu/EasyGameUI/UINavigation/BPI_InputNavigation.NewInputActionTriggered` _output InputType ActionValue))))

(fn `OpenOptionsMenu`
  (returns (`Return Value` :type "/Game/EasyOptionsMenu/Core/WBP_EasyOptionsMenuMain Object Reference"))
  (locals (OptionsMenuWidgetClass :type "UserWidget Object Reference" :default "/Script/UMG.WidgetBlueprintGeneratedClass'/Game/EasyOptionsMenu/Core/WBP_EasyOptionsMenuMain.WBP_EasyOptionsMenuMain_C'"))
  (bind _optionsmenuref (`self.OptionsMenuRef`))
  (bind _optionsmenuwidgetclass (`local.OptionsMenuWidgetClass`))
  (`self.OptionsMenuRef`
    (:`then`
      _)
    (:`else`
      (bind _foundwidgets (`WidgetBlueprintLibrary.GetAllWidgetsOfClass` _optionsmenuwidgetclass false))
      (if (`KismetArrayLibrary.Array_IsNotEmpty` _foundwidgets)
        (set `self.OptionsMenuRef` (`|GetArrayItem` _foundwidgets))
        (else
          (bind _returnvalue (`|CreateWidget` _optionsmenuwidgetclass))
          (set `self.OptionsMenuRef` _returnvalue)))))
  (if (not (`Widget.IsInViewport` _optionsmenuref))
    (`UserWidget.AddToViewport` _optionsmenuref 0))
  (message `/Game/EasyOptionsMenu/EasyGameUI/Utilities/BPI_EGUI_WidgetsCommunicationInterface.SelectInitialOptionsMenuTab` (`self.OptionsMenuRef`) (`self.LastOpenedOptionsMenuTab`))
  (bind _aswbp_easy_options_menu_main (cast `/Game/EasyOptionsMenu/Core/WBP_EasyOptionsMenuMain` (`self.OptionsMenuRef`)))
  (return _aswbp_easy_options_menu_main))

(fn `OpenPauseMenu`
  (returns (`Return Value` :type "UserWidget Object Reference"))
  (bind _widgetref (`/Game/EasyOptionsMenu/EasyGameUI/Utilities/BFL_EasyFunctionUtilities.SafeCreateWidget` "/Game/EasyOptionsMenu/DemoContent/WBP_DemoPauseMenu.WBP_DemoPauseMenu_C" 99))
  (bind _aswbp_demo_pause_menu (cast `/Game/EasyOptionsMenu/DemoContent/WBP_DemoPauseMenu` _widgetref))
  (add `/Game/EasyOptionsMenu/DemoContent/WBP_DemoPauseMenu.PauseMenuClosed` _aswbp_demo_pause_menu (`|CreateDelegate` :!event `RestoreRemovedGameplayMappingContexts`))
  (`/Game/EasyOptionsMenu/EasyGameUI/Utilities/BPI_EGUI_HUDInterface.RemoveAllGameplayInputMappingContexts`)
  (return _widgetref))

(fn `SaveUserSettingsToDisk`
  (returns (`Success?` :type Boolean))
  (bind _returnvalue (`JsonBlueprintFunctionLibrary.ToFile` (`self.GlobalUserSettings`) (`/Game/EasyOptionsMenu/EasyGameUI/Utilities/BFL_EasyFunctionUtilities.GetSettingsFilePath`)))
  (return _returnvalue))

(fn `SetupAlertBanner`
  (params (UnderlyingWidget :type "UserWidget Object Reference") (AlertBannerSetupInfos :type "/Game/EasyOptionsMenu/EasyGameUI/Datas/S_AlertBannerSetupInfos Structure") (`IsInputModeGameAndUI?` :type Boolean))
  (returns (BannerWidget :type "/Game/EasyOptionsMenu/EasyGameUI/CommonWidgets/WBP_EGUI_CommonAlertBanner Object Reference"))
  (bind _alertbannerreference (`self.AlertBannerReference`))
  (bind _output (`|ConvertAsset` (`local.UnderlyingWidget`)))
  (`Widget.SetVisibility` UnderlyingWidget "HitTestInvisible")
  (set `self.RestoreAsInputListener?` (`KismetArrayLibrary.Array_Contains` (`self.InputListeningWidgets`) _output))
  (`/Game/EasyOptionsMenu/EasyGameUI/Utilities/BPI_EGUI_HUDInterface.UnregisterInputListener` _output)
  (bind _alertbannerreference_2 (`self.AlertBannerReference`)
    (:`then`
      (if (`Widget.IsInViewport` _alertbannerreference_2)
        (`Widget.SetVisibility` _alertbannerreference "SelfHitTestInvisible")
        (else
          (`UserWidget.AddToViewport` _alertbannerreference 999 :!label _label))))
    (:`else`
      (bind _returnvalue (`|CreateWidget` "/Game/EasyOptionsMenu/EasyGameUI/CommonWidgets/WBP_EGUI_CommonAlertBanner.WBP_EGUI_CommonAlertBanner_C" null self))
      (set `self.AlertBannerReference` _returnvalue)
      (goto _label)))
  (bind _buttontofocus (`/Game/EasyOptionsMenu/EasyGameUI/CommonWidgets/WBP_EGUI_CommonAlertBanner.SetupWidget` (`self.AlertBannerReference`) (`local.AlertBannerSetupInfos`)))
  (`/Game/EasyOptionsMenu/EasyGameUI/Utilities/BPI_EGUI_HUDInterface.InitializeFocusHandling` (`self.AlertBannerReference`) _buttontofocus true (not (`local.IsInputModeGameAndUI?`)))
  (return (`self.AlertBannerReference`)))

(fn `UpdatePlayerCameraFOV`
  (returns (AppliedFOV :type "Float (double-precision)"))
  (locals (`SelectCustomCamera?` :type Boolean) (CameraReference :type "CameraComponent Object Reference"))
  ;[1 1 1] If the camera selected is not the correct one, set the value of the "Select Custom Camera?" bool to True and add your own code in the "True" pin of the branch to retrieve the proper camera by setting the "Camera Reference" variable.
  (if (not (`local.SelectCustomCamera?`))
    (set `local.CameraReference` (`self.GetComponentByClass` (`self.GetOwningPawn`) "/Script/Engine.CameraComponent")))
  (bind _camerareference (`local.CameraReference`)
    (:`then`
      (bind (_outvalue _returnvalue) (`|GetJsonField` (`self.GlobalUserSettings`) "Camera FOV"))
      (if _returnvalue
        (`CameraComponent.SetFieldOfView` _camerareference _outvalue)
        (return _outvalue)
        (else
          (`CameraComponent.SetFieldOfView` _camerareference 90.0)
          (return 90.0))))
    (:`else`)))

(fn `UserConstructionScript`)