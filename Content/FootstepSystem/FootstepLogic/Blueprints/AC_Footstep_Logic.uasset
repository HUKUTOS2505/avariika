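; Footstep logic component that plays surface-dependent sounds, decals and particles for a character's steps.
; ExcecuteFootstepLogic line-traces vertically around the foot or root socket chosen by notify type, reading the physical surface and impact point.
; On a hit it plays a sound by footstep type and surface, with an optional water-splash layer off water.
; It also spawns left/right decals on sand and snow, plus a surface particle.
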(fn `ExcecuteFootstepLogic`
  (params (`Skeletal Mesh Component` :type "SkeletalMeshComponent Object Reference") (`Footstep Type` :type "/Game/ResourcePack/Animations/Notifies/Enums/Enum_Walk_Types Enum" :default "NewEnumerator0") (`Notify Type` :type "/Game/ResourcePack/Animations/Notifies/Enums/Enum_Notify_Type Enum" :default "NewEnumerator0"))
  ;[1 1 1] Checks the surface based on line trace
  (bind (_has_hit_on_surface _surfacetype _stepimpactlocation) (`self.SurfaceTypeCheck` `Skeletal Mesh Component` `Notify Type`))
  ;[1 1 1] If there is a hit conintue
  (if _has_hit_on_surface
    (`|ExecutionSequence`
      (:`then_0`
        ;[1 1 1] Play sound, spawn decal and spawn footstep particle. Easy to add more logic, add a pin in the sequence
        (`self.Play Footstep Sound` `Footstep Type` _surfacetype _stepimpactlocation))
      (:`then_1`
        (`self.SpawnFootstepDecal` _stepimpactlocation _surfacetype `Skeletal Mesh Component` `Notify Type`))
      (:`then_2`
        (`self.SpawnFootstepParticle` _stepimpactlocation _surfacetype)))))

(fn `Get Footstep Water Splash Sound Based On Footstep Type`
  (params (`Footstep type` :type "/Game/ResourcePack/Animations/Notifies/Enums/Enum_Walk_Types Enum" :default "NewEnumerator0"))
  (returns (`Run Sound` :type "SoundCue Object Reference"))
  (bind _run_footstep_sound_water (`self.Run Footstep Sound Water`))
  (return (select `/Game/ResourcePack/Animations/Notifies/Enums/Enum_Walk_Types` `Footstep type` :`NewEnumerator0` _run_footstep_sound_water :`NewEnumerator1` _run_footstep_sound_water :`NewEnumerator2` _run_footstep_sound_water :`NewEnumerator3` _run_footstep_sound_water :`NewEnumerator4` (`self.Jump Footstep Sound Water`) :`NewEnumerator5` (`self.Land Footstep Sound Water`))))

(fn `Get Jump Sound Based On SurfaceType`
  (params (`Physical surface Type` :type "EPhysicalSurface Enum" :default "SurfaceType_Default"))
  (returns (`Run Sound` :type "SoundCue Object Reference"))
  (return (select `EPhysicalSurface` `Physical surface Type` :`SurfaceType_Default` (`self.Jump Footstep Sound Default`) :`SurfaceType1` (`self.Jump Footstep Sound Grass`) :`SurfaceType2` (`self.Jump Footstep Sound Rock`) :`SurfaceType3` (`self.Jump Footstep Sound Wood`) :`SurfaceType4` (`self.Jump Footstep Sound Water`) :`SurfaceType5` (`self.Jump Footstep Sound Sand`) :`SurfaceType6` (`self.Jump Footstep Sound Snow`) :`SurfaceType7` (`self.Jump Footstep Sound Cloth`))))

(fn `Get Land Sound Based On SurfaceType`
  (params (`Physical surface Type` :type "EPhysicalSurface Enum" :default "SurfaceType_Default"))
  (returns (`Run Sound` :type "SoundCue Object Reference"))
  (return (select `EPhysicalSurface` `Physical surface Type` :`SurfaceType_Default` (`self.Land Footstep Sound Default`) :`SurfaceType1` (`self.Land Footstep Sound Grass`) :`SurfaceType2` (`self.Land Footstep Sound Rock`) :`SurfaceType3` (`self.Land Footstep Sound Wood`) :`SurfaceType4` (`self.Land Footstep Sound Water`) :`SurfaceType5` (`self.Land Footstep Sound Sand`) :`SurfaceType6` (`self.Land Footstep Sound Snow`) :`SurfaceType7` (`self.Land Footstep Sound Cloth`))))

(fn `Get Run Sound Based On SurfaceType`
  (params (`Physical surface Type` :type "EPhysicalSurface Enum" :default "SurfaceType_Default"))
  (returns (`Run Sound` :type "SoundCue Object Reference"))
  (return (select `EPhysicalSurface` `Physical surface Type` :`SurfaceType_Default` (`self.Run Footstep Sound Default`) :`SurfaceType1` (`self.Run Footstep Sound Grass`) :`SurfaceType2` (`self.Run Footstep Sound Rock`) :`SurfaceType3` (`self.Run Footstep Sound Wood`) :`SurfaceType4` (`self.Run Footstep Sound Water`) :`SurfaceType5` (`self.Run Footstep Sound Sand`) :`SurfaceType6` (`self.Run Footstep Sound Snow`) :`SurfaceType7` (`self.Run Footstep Sound Cloth`))))

(fn `GetNotifyLocationBasedOnSocket`
  (params (`Skeletal Mesh Component` :type "SkeletalMeshComponent Object Reference") (`Notify Type` :type "/Game/ResourcePack/Animations/Notifies/Enums/Enum_Notify_Type Enum" :default "NewEnumerator0"))
  (returns (ReturnValue :type "Vector Structure"))
  (switch `/Game/ResourcePack/Animations/Notifies/Enums/Enum_Notify_Type` `Notify Type`
    (:`NewEnumerator0`
      (return (`SceneComponent.GetSocketLocation` `Skeletal Mesh Component` "foot_l")))
    (:`NewEnumerator1`
      (return (`SceneComponent.GetSocketLocation` `Skeletal Mesh Component` "foot_r")))
    (:`NewEnumerator2`
      (return (`SceneComponent.GetSocketLocation` `Skeletal Mesh Component` "root")))))

(fn `GetWalkSoundBasedOnSurfaceType`
  (params (`Physical surface Type` :type "EPhysicalSurface Enum" :default "SurfaceType_Default"))
  (returns (`Run Sound` :type "SoundCue Object Reference"))
  (return (select `EPhysicalSurface` `Physical surface Type` :`SurfaceType_Default` (`self.Walk Footstep sounds default`) :`SurfaceType1` (`self.Walk Footstep sounds Grass`) :`SurfaceType2` (`self.Walk Footstep sounds  Rock`) :`SurfaceType3` (`self.Walk Footstep sounds Wood`) :`SurfaceType4` (`self.Walk Footstep sounds Water`) :`SurfaceType5` (`self.Walk Footstep sounds Sand`) :`SurfaceType6` (`self.Walk Footstep sounds Snow`) :`SurfaceType7` (`self.Walk Footstep sounds Cloth`))))

(fn `Play Footstep Sound`
  (params (`Footstep Type` :type "/Game/ResourcePack/Animations/Notifies/Enums/Enum_Walk_Types Enum" :default "NewEnumerator0") (`Physical surface Type` :type "EPhysicalSurface Enum" :default "SurfaceType_Default") (Location :type "Vector Structure"))
  (bind _run_sound (`self.Get Footstep Water Splash Sound Based On Footstep Type` `Footstep Type`))
  (bind _splash_sound_volume_multiplier (`self.Splash Sound volume multiplier`))
  (switch `/Game/ResourcePack/Animations/Notifies/Enums/Enum_Walk_Types` `Footstep Type`
    (:`NewEnumerator0`
      (`GameplayStatics.PlaySoundAtLocation` (`self.GetWalkSoundBasedOnSurfaceType` `Physical surface Type`) Location (struct) 1.0 1.0 0.0 null null null)
      ;[1 1 1] If surface type is same as water don't spawn water splash sound (otherwise double)
      (if (not (`|EnumEquality` `Physical surface Type` "SurfaceType4"))
        ;[1 1 1] Only play water splash sound when this is enabled. For instance when wet or walking in puddles. This boolean can be set in from the character via the footstep component
        (if (`self.footstep water splash sound enabled`)
          (`GameplayStatics.PlaySoundAtLocation` _run_sound Location (struct) 1.0 1.0 0.0 null null null))))
    (:`NewEnumerator1`
      (`GameplayStatics.PlaySoundAtLocation` (`self.Get Run Sound Based On SurfaceType` `Physical surface Type`) Location (struct) 1.0 1.0 0.0 null null null :!label _label)
      (if (`|EnumEquality` `Physical surface Type` "SurfaceType4")
        _
        (elif (`self.footstep water splash sound enabled`)
          (`GameplayStatics.PlaySoundAtLocation` _run_sound Location (struct) _splash_sound_volume_multiplier 1.0 0.0 null null null))))
    (:`NewEnumerator2`
      (goto _label))
    (:`NewEnumerator3`
      (goto _label))
    (:`NewEnumerator4`
      (`GameplayStatics.PlaySoundAtLocation` (`self.Get Jump Sound Based On SurfaceType` `Physical surface Type`) Location (struct) 1.0 1.0 0.0 null null null)
      (if (`|EnumEquality` `Physical surface Type` "SurfaceType4")
        _
        (elif (`self.footstep water splash sound enabled`)
          (`GameplayStatics.PlaySoundAtLocation` _run_sound Location (struct) _splash_sound_volume_multiplier 1.0 0.0 null null null))))
    (:`NewEnumerator5`
      (`GameplayStatics.PlaySoundAtLocation` (`self.Get Land Sound Based On SurfaceType` `Physical surface Type`) Location (struct) 1.0 1.0 0.0 null null null)
      (if (`|EnumEquality` `Physical surface Type` "SurfaceType4")
        _
        (elif (`self.footstep water splash sound enabled`)
          (`GameplayStatics.PlaySoundAtLocation` _run_sound Location (struct) _splash_sound_volume_multiplier 1.0 0.0 null null null))))))

(fn `SpawnFootstepDecal`
  (params (NotifyLocation :type "Vector Structure") (`Physical Surface Type` :type "EPhysicalSurface Enum" :default "SurfaceType_Default") (`Skeletal Mesh Component` :type "SkeletalMeshComponent Object Reference") (`Notify Type` :type "/Game/ResourcePack/Animations/Notifies/Enums/Enum_Notify_Type Enum" :default "NewEnumerator0"))
  (locals (`Local stored footstep Decal left` :type "MaterialInterface Object Reference") (`Local stored footstep Decal right` :type "MaterialInterface Object Reference"))
  (bind (_returnvalue_roll _returnvalue_pitch _returnvalue_yaw) (`KismetMathLibrary.BreakRotator` (`Actor.K2_GetActorRotation` (`self.GetOwner` `Skeletal Mesh Component`))))
  (switch `/Game/ResourcePack/Animations/Notifies/Enums/Enum_Notify_Type` `Notify Type`
    (:`NewEnumerator0`
      (switch `EPhysicalSurface` `Physical Surface Type`
        (:`SurfaceType5`
          ;[1 1 1] Switches decal based on surface type. If none defined, none spawned.
          (set `local.Local stored footstep Decal left` (`self.Sand footstep Decal left`)))
        (:`SurfaceType6`
          (set `local.Local stored footstep Decal left` (`self.Snow footstep decal left`))))
      (`GameplayStatics.SpawnDecalAtLocation` (`local.Local stored footstep Decal left`) (50.0 20.0 -20.0) NotifyLocation (`KismetMathLibrary.MakeRotator` -90.0 90.0 _returnvalue_yaw) (`self.Footstep decal life`)))
    (:`NewEnumerator1`
      (switch `EPhysicalSurface` `Physical Surface Type`
        (:`SurfaceType5`
          ;[1 1 1] Switches decal based on surface type. If none defined, none spawned.
          (set `local.Local stored footstep Decal right` (`self.Sand footstep Decal Right`)))
        (:`SurfaceType6`
          (set `local.Local stored footstep Decal right` (`self.Snow footstep Decal Right`))))
      (`GameplayStatics.SpawnDecalAtLocation` (`local.Local stored footstep Decal right`) (50.0 20.0 -20.0) NotifyLocation (`KismetMathLibrary.MakeRotator` -90.0 90.0 _returnvalue_yaw) (`self.Footstep decal life`)))))

(fn `SpawnFootstepParticle`
  (params (Location :type "Vector Structure") (`Physical Surface Type` :type "EPhysicalSurface Enum" :default "SurfaceType_Default"))
  (locals (`Local footstep particle` :type "ParticleSystem Object Reference"))
  ;[1 1 1] Switches particle based on surface type. If none defined, none spawned.
  (switch `EPhysicalSurface` `Physical Surface Type`
    (:`SurfaceType_Default`
      (set `local.Local footstep particle` (`self.GenericDust`) :!label _label))
    (:`SurfaceType1`
      (set `local.Local footstep particle` (`self.Grass footstep particle`)))
    (:`SurfaceType2`
      (goto _label))
    (:`SurfaceType3`
      (goto _label))
    (:`SurfaceType4`
      (set `local.Local footstep particle` (`self.Water footstep particle`)))
    (:`SurfaceType5`
      (set `local.Local footstep particle` (`self.Sand footstep particle`)))
    (:`SurfaceType6`
      (set `local.Local footstep particle` (`self.Snow footstep particle`))))
  (`GameplayStatics.SpawnEmitterAtLocation` (`local.Local footstep particle`) Location))

(fn `SurfaceTypeCheck`
  (params (`Skeletal Mesh Component` :type "SkeletalMeshComponent Object Reference") (`Notify Type` :type "/Game/ResourcePack/Animations/Notifies/Enums/Enum_Notify_Type Enum" :default "NewEnumerator0"))
  (returns (`Has Hit On Surface` :type Boolean) (SurfaceType :type "EPhysicalSurface Enum") (StepImpactLocation :type "Vector Structure"))
  ;[1 1 1] Gets the location from foot socket position
  (bind _returnvalue (`self.GetNotifyLocationBasedOnSocket` `Skeletal Mesh Component` `Notify Type`))
  ;[1 1 1] Line trace from the foot location.
  ; We want to know the surface type on which the foot hits. This can be found in the physical material reference.
  ; We also want to know the location of the hit for particle and print effects.
  (bind (_outhit _returnvalue_2) (`KismetSystemLibrary.LineTraceSingle` (+ _returnvalue (0.0 0.0 45.0)) (- _returnvalue (0.0 0.0 45.0)) "TraceTypeQuery1"))
  (if _returnvalue_2
    ;[1 1 1] If there is a hit, return the surface type, location and true state
    (return true (`GameplayStatics.GetSurfaceType` _outhit) (`.Location` (`GameplayStatics.BreakHitResult` _outhit)))
    (else
      ;[1 1 1] If there is no hit, return false
      (return false "SurfaceType_Default" (0.0 0.0 0.0)))))