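; BP_TEST is a test actor that exercises validity checks on a Text Render component.
; BeginPlay destroys the TextRender component.
; Each actor overlap increments TextSize, then applies that size and NewText if TextRender is valid.
; Otherwise it prints the Russian error string "Ошибка", the expected branch once the component is destroyed.
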(event `self.ReceiveBeginPlay`
  (`ActorComponent.K2_DestroyComponent` (`self.TextRender`)))

(event `self.ReceiveActorBeginOverlap`
  (params (OtherActor :type "Actor Object Reference"))
  (bind _textrender (`self.TextRender`))
  (bind _output_get (set `self.TextSize` (+ (`self.TextSize`) 20.0)))
  (`/Engine/EditorBlueprintResources/StandardMacros.IsValid` _textrender
    (:`Is Valid`
      (`TextRenderComponent.SetWorldSize` _textrender _output_get)
      (`TextRenderComponent.K2_SetText` _textrender (`self.New text`)))
    (:`Is Not Valid`
      (`KismetSystemLibrary.PrintString` "Ошибка"))))

(fn `UserConstructionScript`)